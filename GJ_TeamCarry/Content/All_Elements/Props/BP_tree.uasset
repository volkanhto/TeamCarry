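; BP_tree is a tree prop assembled in the Construction Script, with no active runtime logic.
; It adds one Instanced Static Mesh instance at the origin, then attaches a child actor 550 units above with stepped random roll, pitch and yaw for variety.
; Randomness is unseeded, so the rotation re-rolls whenever construction runs; leftover random rotation and scale nodes are unconnected.
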(fn `UserConstructionScript`
  (`|ExecutionSequence`
    (:`then_0`
      (`InstancedStaticMeshComponent.AddInstance` (`self.InstancedStaticMesh`) (`KismetMathLibrary.MakeTransform` (0.0 0.0 0.0))))
    (:`then_1`
      (`AddComponent|NODE_AddChildActorComponent-0` :`RelativeTransform` (`KismetMathLibrary.MakeTransform` (0.0 0.0 550.0) (`KismetMathLibrary.MakeRotator` (* (`KismetMathLibrary.RandomInteger` 2) 10.0) (* (`KismetMathLibrary.RandomInteger` 4) 5.0) (* (`KismetMathLibrary.RandomInteger` 8) 15.0)))))))